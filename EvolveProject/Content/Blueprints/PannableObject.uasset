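; PannableObject is an actor that can be switched on and off in place, with no spawn or destroy logic of its own.
; SetActive stores the Active flag and toggles visibility, ticking and collision together, while GetActive reports the flag.
; ActivateAt teleports the actor to a given location without sweeping, then activates it.
; The event graph and construction script are empty.
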(event `self.ReceiveBeginPlay`)

(event `self.ReceiveActorBeginOverlap`
  (params (OtherActor :type "Actor Object Reference")))

(event `self.ReceiveTick`
  (params (DeltaSeconds :type "Float (single-precision)")))

(fn `ActivateAt`
  (params (Location :type "Object.Vector Structure"))
  (`self.K2_SetActorLocation` Location)
  (`self.SetActive` true))

(fn `GetActive`
  (returns (Active :type Boolean))
  (return (`self.Active`)))

(fn `SetActive`
  (params (Active :type Boolean))
  (bind _output_get (set `self.Active` Active))
  (`self.SetActorHiddenInGame` (not _output_get))
  (`self.SetActorTickEnabled` _output_get)
  (`self.SetActorEnableCollision` _output_get))

(fn `UserConstructionScript`)