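; ObjectPlacer is an actor that places objects at fixed intervals along world Y as its own position advances in that direction.
; Each Tick compares its Y with LastSpawn, seeded in the construction script, and once SpawnIntensity is reached picks a random entry from the SpawnActors pool.
; An inactive pick is activated at the exact interval position, independent of overshoot, and LastSpawn advances; an active pick leaves placement to a later Tick.
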(event `self.ReceiveBeginPlay`)

(event `self.ReceiveActorBeginOverlap`
  (params (OtherActor :type "Actor Object Reference")))

(event `self.ReceiveTick`
  (params (DeltaSeconds :type "Float (single-precision)"))
  (bind _spawnactors (`self.SpawnActors`))
  (bind _item (`KismetArrayLibrary.Array_Get` _spawnactors (`self.NextToSpawn`)))
  (bind _returnvalue (+ (`self.LastSpawn`) (`self.SpawnIntensity`)))
  (`parent.ReceiveTick` DeltaSeconds)
  ;[1 1 1] Update distance traveled.
  (set `self.DistanceSinceSpawn` (- (.y (`self.K2_GetActorLocation`)) (`self.LastSpawn`)))
  (if (>= (`self.DistanceSinceSpawn`) (`self.SpawnIntensity`))
    ;[1 1 1] Spawn one random Actor
    (set `self.NextToSpawn` (`KismetMathLibrary.RandomIntegerInRange` 0 (- (`KismetArrayLibrary.Array_Length` _spawnactors) 1)))
    (bind _active (`/Game/Blueprints/PannableObject.GetActive` _item))
    (if (not _active)
      (`/Game/Blueprints/PannableObject.ActivateAt` _item (`KismetMathLibrary.MakeVector` (.x (`self.K2_GetActorLocation`)) _returnvalue (.z (`self.K2_GetActorLocation`))))
      (set `self.LastSpawn` _returnvalue))))

(fn `UserConstructionScript`
  (`parent.UserConstructionScript`)
  (set `self.LastSpawn` (.y (`self.K2_GetActorLocation`))))