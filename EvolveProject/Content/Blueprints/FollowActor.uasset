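; FollowActor moves itself each Tick to follow a Target actor's location on chosen axes only.
; The Axes and AxesInverse vectors mask a blend of Target location plus Offset with its own location, set without sweep.
; The construction script sets and prints Offset, commented as own minus target position, though both location reads as written name no Target.
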(event `self.ReceiveBeginPlay`)

(event `self.ReceiveActorBeginOverlap`
  (params (OtherActor :type "Actor Object Reference")))

(event `self.ReceiveTick`
  (params (DeltaSeconds :type "Float (single-precision)"))
  ;[1 1 1] Set my position to the targets position (only the chosen axes)
  (`self.K2_SetActorLocation` (+ (* (`self.K2_GetActorLocation`) (`self.AxesInverse`)) (* (+ (`self.Offset`) (`self.K2_GetActorLocation` (`self.Target`))) (`self.Axes`)))))

(fn `UserConstructionScript`
  ;[1 1 1] Set Offset to MyPos - TargetPos
  (bind _output_get (set `self.Offset` (- (`self.K2_GetActorLocation`) (`self.K2_GetActorLocation`))))
  (`KismetSystemLibrary.PrintString` (`KismetStringLibrary.Conv_VectorToString` _output_get)))